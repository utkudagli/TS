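; First-person player weapon Blueprint covering ten guns, with firing, ammo and reloading.
; FireBullet spawns a projectile from the barrel along the owning player's camera rotation, decrements ammo and calls FireAnim; StartShooting and StopShooting only toggle IsFiring.
; FireAnim and ReloadAnim branch on GunName for arm and gun animations, plus camera shakes for non-pistols.
; Reload refills from reserve ammo; shotgun shell animations loop without delays.
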(event Custom|StartShooting
  (Variables|Default|SetIsFiring true))

(event Custom|StopShooting
  (Variables|Default|SetIsFiring false))

(fn ConstructionScript)

(fn FireBullet
  (bind _asbp_player (Utilities|Casting|CastToBP_Player (Actor|GetParentActor)))
  (if (> (Variables|Default|GetAmmoCount) 0)
    (Game|SpawnActorfromClass "/Game/FirstPersonBP/Blueprints/FirstPersonProjectile.FirstPersonProjectile_C" (Math|Transform|MakeTransform (Transformation|GetWorldLocation (Variables|Default|GetBarrel)) (Transformation|GetWorldRotation (Variables|/Game/Blueprints/BP_Player.BP_Player_C|GetFirstPersonCamera _asbp_player)) "1,1,1") "Undefined" 0 0)
    (CallFunction|FireAnim)
    (Math|Integer|DecrementInt (Variables|Default|GetAmmoCount))))

(fn FireAnim
  (if (Utilities|Enum|Equal(Enum) (Variables|Default|GetGunName) (Utilities|Array|Get(acopy) (Variables|Default|GetWeaponList)))
    (Components|Animation|PlayAnimation (Variables|Default|GetArms) "/Game/Animations/FPP/Machinery/AK74/AK74_Arm_Fire_Start.AK74_Arm_Fire_Start" false)
    (Components|Animation|PlayAnimation (Variables|Default|GetBase) "/Game/Weapons/Base/Machines/AK47/Anim/AK74_Fire_Start.AK74_Fire_Start" false)
    (Camera|PlayWorldCameraShake "/Game/Effects/BP_RifleShake.BP_RifleShake_C" (Transformation|GetActorLocation (Game|Player|GetPlayerPawn 0)) 0.0 5e+02 :!label _label)
    (elif (Utilities|Enum|Equal(Enum) (Variables|Default|GetGunName) (Utilities|Array|Get(acopy) (Variables|Default|GetWeaponList) 1))
      (Components|Animation|PlayAnimation (Variables|Default|GetArms) "/Game/Animations/FPP/Machinery/AUG_EF88/AUG_Arm_Fire_Start.AUG_Arm_Fire_Start" false)
      (Components|Animation|PlayAnimation (Variables|Default|GetBase) "/Game/Weapons/Base/Machines/AUG_EF88/Anim/AUG_Fire_Start.AUG_Fire_Start" false)
      (goto _label)
      (elif (Utilities|Enum|Equal(Enum) (Variables|Default|GetGunName) (Utilities|Array|Get(acopy) (Variables|Default|GetWeaponList) 2))
        (Components|Animation|PlayAnimation (Variables|Default|GetArms) "/Game/Animations/FPP/Pistols/Glock19/Glock19_Arm_Fire_End.Glock19_Arm_Fire_End" false)
        (Components|Animation|PlayAnimation (Variables|Default|GetBase) "/Game/Weapons/Base/Pistols/Glock19/Anim/Glock19_Fire_Start.Glock19_Fire_Start" false)
        (elif (Utilities|Enum|Equal(Enum) (Variables|Default|GetGunName) (Utilities|Array|Get(acopy) (Variables|Default|GetWeaponList) 3))
          (Components|Animation|PlayAnimation (Variables|Default|GetArms) "/Game/Animations/FPP/Pistols/DEagle/DEagle_Arm_Fire_Start.DEagle_Arm_Fire_Start" false)
          (Components|Animation|PlayAnimation (Variables|Default|GetBase) "/Game/Weapons/Base/Pistols/DEagle/Anim/DEagle_Fire_Start.DEagle_Fire_Start" false)
          (elif (Utilities|Enum|Equal(Enum) (Variables|Default|GetGunName) (Utilities|Array|Get(acopy) (Variables|Default|GetWeaponList) 4))
            (Components|Animation|PlayAnimation (Variables|Default|GetArms) "/Game/Animations/FPP/Snipers/AWP/Awp_Arm_Fire.Awp_Arm_Fire" false)
            (Components|Animation|PlayAnimation (Variables|Default|GetBase) "/Game/Weapons/Base/Snipers/AWP/Anim/Awp_Fire.Awp_Fire" false)
            (Camera|PlayWorldCameraShake "/Game/Effects/BP_SniperShake.BP_SniperShake_C" (Transformation|GetActorLocation (Game|Player|GetPlayerPawn 0)) 0.0 5e+02 :!label _label_2)
            (elif (Utilities|Enum|Equal(Enum) (Variables|Default|GetGunName) (Utilities|Array|Get(acopy) (Variables|Default|GetWeaponList) 5))
              (Components|Animation|PlayAnimation (Variables|Default|GetArms) "/Game/Animations/FPP/Snipers/KNT76/KNT76_Arm_Fire_Start.KNT76_Arm_Fire_Start" false)
              (goto _label_2)
              (elif (Utilities|Enum|Equal(Enum) (Variables|Default|GetGunName) (Utilities|Array|Get(acopy) (Variables|Default|GetWeaponList) 6))
                (Components|Animation|PlayAnimation (Variables|Default|GetArms) "/Game/Animations/FPP/LightMachines/KrissVector/KrissVector_Arm_Fire_Start.KrissVector_Arm_Fire_Start" false)
                (Components|Animation|PlayAnimation (Variables|Default|GetBase) "/Game/Weapons/Base/LightMachines/KrissVector/Anim/KrissVector_Fire_Start.KrissVector_Fire_Start" false)
                (Camera|PlayWorldCameraShake "/Game/Effects/BP_LightMahineShake.BP_LightMahineShake_C" (Transformation|GetActorLocation (Game|Player|GetPlayerPawn 0)) 0.0 5e+02 :!label _label_3)
                (elif (Utilities|Enum|Equal(Enum) (Variables|Default|GetGunName) (Utilities|Array|Get(acopy) (Variables|Default|GetWeaponList) 7))
                  (Components|Animation|PlayAnimation (Variables|Default|GetArms) "/Game/Animations/FPP/LightMachines/UMP/UMP_Arm_Fire_Start.UMP_Arm_Fire_Start" false)
                  (Components|Animation|PlayAnimation (Variables|Default|GetBase) "/Game/Weapons/Base/LightMachines/UMP/Anim/UMP_Fire_Start.UMP_Fire_Start" false)
                  (goto _label_3)
                  (elif (Utilities|Enum|Equal(Enum) (Variables|Default|GetGunName) (Utilities|Array|Get(acopy) (Variables|Default|GetWeaponList) 8))
                    (Components|Animation|PlayAnimation (Variables|Default|GetArms) "/Game/Animations/FPP/Shotguns/Nova/Nova_Arm_Fire_Start.Nova_Arm_Fire_Start" false)
                    (Components|Animation|PlayAnimation (Variables|Default|GetBase) "/Game/Weapons/Base/Shotguns/Nova/Anim/Nova_Fire_Start.Nova_Fire_Start" false)
                    (Camera|PlayWorldCameraShake "/Game/Effects/BP_ShotgunShake.BP_ShotgunShake_C" (Transformation|GetActorLocation (Game|Player|GetPlayerPawn 0)) 0.0 5e+02 1.0 true :!label _label_4)
                    (elif (Utilities|Enum|Equal(Enum) (Variables|Default|GetGunName) (Utilities|Array|Get(acopy) (Variables|Default|GetWeaponList) 9))
                      (Components|Animation|PlayAnimation (Variables|Default|GetArms) "/Game/Animations/FPP/Shotguns/UTS15/UTS15_Arm_Fire_Start.UTS15_Arm_Fire_Start" false)
                      (Components|Animation|PlayAnimation (Variables|Default|GetBase) "/Game/Weapons/Base/Shotguns/UTS15/Anim/UTS15_Fire_Start.UTS15_Fire_Start" false)
                      (goto _label_4))))))))))))

(fn Reload
  (CallFunction|ReloadAnim)
  (bind _output_get (LocalVariables|SetBulletDiffrence (- (Variables|Default|GetClipSize) (Variables|Default|GetAmmoCount))))
  (if (>= (Variables|Default|GetAmmoMax) _output_get)
    (Variables|Default|SetAmmoCount (Variables|Default|GetClipSize))
    (Variables|Default|SetAmmoMax (- (Variables|Default|GetAmmoMax) (LocalVariables|GetBulletDiffrence)))
    (else
      (Variables|Default|SetAmmoCount (+ (Variables|Default|GetAmmoCount) (Variables|Default|GetAmmoMax)))
      (Variables|Default|SetAmmoMax 0))))

(fn ReloadAnim
  (if (Utilities|Enum|Equal(Enum) (Variables|Default|GetGunName) (Utilities|Array|Get(acopy) (Variables|Default|GetWeaponList)))
    (Components|Animation|PlayAnimation (Variables|Default|GetArms) "/Game/Animations/FPP/Machinery/AK74/AK74_Arm_Reload.AK74_Arm_Reload" false)
    (Components|Animation|PlayAnimation (Variables|Default|GetBase) "/Game/Weapons/Base/Machines/AK47/Anim/AK74_Reload.AK74_Reload" false)
    (elif (Utilities|Enum|Equal(Enum) (Variables|Default|GetGunName) (Utilities|Array|Get(acopy) (Variables|Default|GetWeaponList) 1))
      (Components|Animation|PlayAnimation (Variables|Default|GetArms) "/Game/Animations/FPP/Machinery/AUG_EF88/AUG_Arm_Reload.AUG_Arm_Reload" false)
      (Components|Animation|PlayAnimation (Variables|Default|GetBase) "/Game/Weapons/Base/Machines/AUG_EF88/Anim/AUG_Reload.AUG_Reload" false)
      (elif (Utilities|Enum|Equal(Enum) (Variables|Default|GetGunName) (Utilities|Array|Get(acopy) (Variables|Default|GetWeaponList) 2))
        (Components|Animation|PlayAnimation (Variables|Default|GetArms) "/Game/Animations/FPP/Pistols/Glock19/Glock19_Arm_Reload.Glock19_Arm_Reload" false)
        (Components|Animation|PlayAnimation (Variables|Default|GetBase) "/Game/Weapons/Base/Pistols/Glock19/Anim/Glock19_Reload.Glock19_Reload" false)
        (elif (Utilities|Enum|Equal(Enum) (Variables|Default|GetGunName) (Utilities|Array|Get(acopy) (Variables|Default|GetWeaponList) 3))
          (Components|Animation|PlayAnimation (Variables|Default|GetArms) "/Game/Animations/FPP/Pistols/DEagle/DEagle_Arm_Reload.DEagle_Arm_Reload" false)
          (Components|Animation|PlayAnimation (Variables|Default|GetBase) "/Game/Weapons/Base/Pistols/DEagle/Anim/DEagle_Reload_Short.DEagle_Reload_Short" false)
          (elif (Utilities|Enum|Equal(Enum) (Variables|Default|GetGunName) (Utilities|Array|Get(acopy) (Variables|Default|GetWeaponList) 4))
            (Components|Animation|PlayAnimation (Variables|Default|GetArms) "/Game/Animations/FPP/Snipers/AWP/Awp_Arm_Reload.Awp_Arm_Reload" false)
            (Components|Animation|PlayAnimation (Variables|Default|GetBase) "/Game/Weapons/Base/Snipers/AWP/Anim/Awp_Reload.Awp_Reload" false)
            (elif (Utilities|Enum|Equal(Enum) (Variables|Default|GetGunName) (Utilities|Array|Get(acopy) (Variables|Default|GetWeaponList) 5))
              (Components|Animation|PlayAnimation (Variables|Default|GetArms) "/Game/Animations/FPP/Snipers/KNT76/KNT76_Arm_Reload.KNT76_Arm_Reload" false)
              (Components|Animation|PlayAnimation (Variables|Default|GetBase) "/Game/Weapons/Base/Snipers/KNT76/Anim/KNT76_Reload.KNT76_Reload" false)
              (elif (Utilities|Enum|Equal(Enum) (Variables|Default|GetGunName) (Utilities|Array|Get(acopy) (Variables|Default|GetWeaponList) 6))
                (Components|Animation|PlayAnimation (Variables|Default|GetArms) "/Game/Animations/FPP/LightMachines/KrissVector/KrissVector_Arm_Reload.KrissVector_Arm_Reload" false)
                (Components|Animation|PlayAnimation (Variables|Default|GetBase) "/Game/Weapons/Base/LightMachines/KrissVector/Anim/KrissVector_Reload.KrissVector_Reload" false)
                (elif (Utilities|Enum|Equal(Enum) (Variables|Default|GetGunName) (Utilities|Array|Get(acopy) (Variables|Default|GetWeaponList) 7))
                  (Components|Animation|PlayAnimation (Variables|Default|GetArms) "/Game/Animations/FPP/LightMachines/UMP/UMP_Arm_Reload.UMP_Arm_Reload" false)
                  (Components|Animation|PlayAnimation (Variables|Default|GetBase) "/Game/Weapons/Base/LightMachines/UMP/Anim/UMP_Reload.UMP_Reload" false)
                  (elif (Utilities|Enum|Equal(Enum) (Variables|Default|GetGunName) (Utilities|Array|Get(acopy) (Variables|Default|GetWeaponList) 8))
                    (Components|Animation|PlayAnimation (Variables|Default|GetArms) "/Game/Animations/FPP/Shotguns/Nova/Nova_Arm_Reload_Start.Nova_Arm_Reload_Start" false)
                    (Components|Animation|PlayAnimation (Variables|Default|GetBase) "/Game/Weapons/Base/Shotguns/Nova/Anim/Nova_Reload_Start.Nova_Reload_Start" false)
                    (Variables|Default|SetCurrent%20Shell (Variables|Default|GetAmmoCount))
                    (if (< (Variables|Default|GetCurrent%20Shell) 7) :!label _label
                      (Components|Animation|PlayAnimation (Variables|Default|GetArms) "/Game/Animations/FPP/Shotguns/Nova/Nova_Arm_Reload_Loop.Nova_Arm_Reload_Loop" false)
                      (Components|Animation|PlayAnimation (Variables|Default|GetBase) "/Game/Weapons/Base/Shotguns/Nova/Anim/Nova_Reload_Loop.Nova_Reload_Loop" false)
                      (Variables|Default|SetCurrent%20Shell (+ (Variables|Default|GetCurrent%20Shell) 1))
                      (if (== (Variables|Default|GetCurrent%20Shell) 7)
                        (Components|Animation|PlayAnimation (Variables|Default|GetArms) "/Game/Animations/FPP/Shotguns/Nova/Nova_Arm_Reload_End.Nova_Arm_Reload_End" false)
                        (Components|Animation|PlayAnimation (Variables|Default|GetBase) "/Game/Weapons/Base/Shotguns/Nova/Anim/Nova_Reload_End.Nova_Reload_End" false)
                        (else
                          (goto _label))))
                    (elif (Utilities|Enum|Equal(Enum) (Variables|Default|GetGunName) (Utilities|Array|Get(acopy) (Variables|Default|GetWeaponList) 9))
                      (Components|Animation|PlayAnimation (Variables|Default|GetArms) "/Game/Animations/FPP/Shotguns/UTS15/UTS15_Arm_Reload_Start.UTS15_Arm_Reload_Start" false)
                      (Components|Animation|PlayAnimation (Variables|Default|GetBase) "/Game/Weapons/Base/Shotguns/UTS15/Anim/UTS15_Reload_Start.UTS15_Reload_Start" false)
                      (Variables|Default|SetCurrent%20Shell (Variables|Default|GetAmmoCount))
                      (if (< (Variables|Default|GetCurrent%20Shell) 7) :!label _label_2
                        (Components|Animation|PlayAnimation (Variables|Default|GetArms) "/Game/Animations/FPP/Shotguns/UTS15/UTS15_Arm_Reload_Loop.UTS15_Arm_Reload_Loop" false)
                        (Components|Animation|PlayAnimation (Variables|Default|GetBase) "/Game/Weapons/Base/Shotguns/UTS15/Anim/UTS15_Reload_Loop.UTS15_Reload_Loop" false)
                        (Variables|Default|SetCurrent%20Shell (+ (Variables|Default|GetCurrent%20Shell) 1))
                        (if (== (Variables|Default|GetCurrent%20Shell) 7)
                          (Components|Animation|PlayAnimation (Variables|Default|GetArms) "/Game/Animations/FPP/Shotguns/UTS15/UTS15_Arm_Reload_End.UTS15_Arm_Reload_End" false)
                          (Components|Animation|PlayAnimation (Variables|Default|GetBase) "/Game/Weapons/Base/Shotguns/UTS15/Anim/UTS15_Reload_End.UTS15_Reload_End" false)
                          (else
                            (goto _label_2)))))))))))))))